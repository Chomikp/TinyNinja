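; Basic enemy character with health, a patrol route and adjustable walk speed.
; Health starts at max on BeginPlay and is printed every Tick as debug output.
; AnyDamage passes through a DoOnce with no reset, so only the first hit subtracts health, destroying the actor if none remains.
; The construction script appends local patrol points converted to world space to a global route, and UpdateWalkSpeed sets movement speed.
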(event Game|Damage|EventAnyDamage
  (params (Damage :type Float%20%28single-precision%29) (DamageType :type Damage%20Type%20Object%20Reference) (InstigatedBy :type Controller%20Object%20Reference) (DamageCauser :type Actor%20Object%20Reference))
  (Utilities|FlowControl|DoOnce false
    (:Completed
      (bind _output_get (Variables|Default|SetCurrentHealth (- (Variables|Default|GetCurrentHealth) Damage)))
      (if (not (> _output_get 0.0))
        (Actor|DestroyActor)))))

(event EventBeginPlay
  (Variables|Default|SetCurrentHealth (Variables|Default|GetMaxHealth)))

(event EventTick
  (params (DeltaSeconds :type Float%20%28single-precision%29))
  (Development|PrintString (Utilities|String|Append (Utilities|GetDisplayName (Variables|Character|GetMesh)) " current health is: " (Utilities|String|ToString(Float) (Variables|Default|GetCurrentHealth))) true true "(R=0.000000,G=0.660000,B=1.000000,A=1.000000)" 0.0))

(fn ConstructionScript
  (for _array_element (Variables|Patrol|GetPatrolRouteLocal)
    (Utilities|Array|Add (Variables|Patrol|GetPatrolRouteGlobal) (Math|Transform|TransformLocation (Transformation|GetActorTransform) _array_element))))

(fn UpdateWalkSpeed
  (params (NewWalkSpeed :type Float%20%28double-precision%29))
  (Variables|/Script/Engine.CharacterMovementComponent|SetMaxWalkSpeed (Variables|Character|GetCharacterMovement) NewWalkSpeed))