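; Test enemy AI controller that uses perception to detect the player and drive a State Tree.
; Sensing a Player-tagged actor stores it, adds a detected gameplay tag, sends a State Tree event and starts a timer that later clears detection.
; A distance check traces to head, chest and groin and writes the longest hit to the Blackboard, but its looping timer setup is disconnected.
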(event OnTargetPerceptionUpdated(AIPerception)
  (params (Actor :type Actor%20Object%20Reference) (Stimulus :type AI%20Stimulus%20Structure))
  (if (Actor|ActorHasTag Actor "Player")
    (Variables|BlackboardValues|SetSensedActor Actor)
    (GameplayTags|AddGameplayTag (Variables|Default|GetGameplayTagContainer) "(TagName=\"Enemy.PlayerDetected\")" :!class /Script/GameplayTags.BlueprintGameplayTagLibrary)
    (Gameplay|StateTree|SendStateTreeEvent (Variables|Default|GetStateTreeAI) (Variables|Default|GetEvent) :!class /Script/GameplayStateTreeModule.StateTreeComponent)
    (bind _returnvalue (Utilities|Time|SetTimerbyEvent (delegate Custom|Clear%20Timer) (Variables|Detection|GetLineOfSightTimer)))
    (Variables|Default|SetLineOfSightTimerHandle _returnvalue)))

(event Custom|Clear%20Timer
  (Utilities|Time|ClearandInvalidateTimerbyHandle (Variables|Default|GetLineOfSightTimerHandle))
  (Variables|BlackboardValues|SetSensedActor 0)
  (GameplayTags|RemoveGameplayTag (Variables|Default|GetGameplayTagContainer) "(TagName=\"Enemy.PlayerDetected\")" :!class /Script/GameplayTags.BlueprintGameplayTagLibrary))

(event Custom|GetDistanceAndStealth
  (bind _sensedactor (Variables|BlackboardValues|GetSensedActor))
  ;[1 1 1] If player is sensed start calculating current distance between enemy and player on a short timer. This needs to be refreshed often so that enemy can react properly and quickly based on distance
  (if (and (== 0 _sensedactor) (Utilities|IsValid _sensedactor))
    (CallFunction|GetDistancetoPlayer)
    (AI|Components|Blackboard|SetValueasFloat (Variables|Default|GetBlackboard) (Variables|BlackboardValues|GetDistanceToPlayer) (Variables|BlackboardValues|GetDistanceToPlayerValue))))

(event EventInDetectionSphere
  (params (OtherActor :type Actor%20Object%20Reference) (InsideRange :type Boolean)))

(event EventCurrentPlayerDetectionRange
  (params (Value :type Float%20%28double-precision%29)))

(event EventPossess
  (params (PossessedPawn :type Pawn%20Object%20Reference))
  (Variables|Default|SetPossesed%20Pawn PossessedPawn))

(fn ConstructionScript)

(fn GetDistancetoPlayer
  (Variables|Detection|SetPawnEyesLocation (+ (Transformation|GetActorLocation (Variables|Default|GetPossesed%20Pawn)) "0.000000,0.000000,45.000000"))
  ;[1 1 1] I use three separate traces to make sure one of them hits. There may be an animation where one part of the body isn't aligned with the middle of mesh and in that instance one trace would miss.
  (Utilities|FlowControl|Sequence
    (:then_0
      ;[1 1 1] Check top of the head
      (bind _outhit (Collision|LineTraceByChannel (Variables|Detection|GetPawnEyesLocation) (+ (Transformation|GetActorLocation (Variables|BlackboardValues|GetSensedActor)) "0.000000,0.000000,60.000000") "TraceTypeQuery2" false 0 "ForDuration" false "(R=1.000000,G=0.000000,B=0.000000,A=1.000000)" "(R=0.000000,G=1.000000,B=0.000000,A=1.000000)" (Variables|Detection|DetectDistance|GetDistanceDetectionFrequency)))
      ;[1 1 1] Reset previous distance and if trace has hit player pawn update it with new value
      (Variables|Detection|DetectDistance|SetDistanceToHead 0.0)
      (if (== (.HitActor (Collision|BreakHitResult _outhit)) (Variables|BlackboardValues|GetSensedActor))
        (Variables|Detection|DetectDistance|SetDistanceToHead (.Distance (Collision|BreakHitResult _outhit)))))
    (:then_1
      ;[1 1 1] Check chest
      (bind _outhit_2 (Collision|LineTraceByChannel (Variables|Detection|GetPawnEyesLocation) (+ (Transformation|GetActorLocation (Variables|BlackboardValues|GetSensedActor)) "") "TraceTypeQuery2" false 0 "ForDuration" true "(R=1.000000,G=0.000000,B=0.000000,A=1.000000)" "(R=0.000000,G=1.000000,B=0.000000,A=1.000000)" (Variables|Detection|DetectDistance|GetDistanceDetectionFrequency)))
      (Variables|Detection|DetectDistance|SetDistanceToChest 0.0)
      (if (== (.HitActor (Collision|BreakHitResult _outhit_2)) (Variables|BlackboardValues|GetSensedActor))
        (Variables|Detection|DetectDistance|SetDistanceToChest (.Distance (Collision|BreakHitResult _outhit_2)))))
    (:then_2
      ;[1 1 1] Check groin
      (bind _outhit_3 (Collision|LineTraceByChannel (Variables|Detection|GetPawnEyesLocation) (+ (Transformation|GetActorLocation (Variables|BlackboardValues|GetSensedActor)) "0.000000,0.000000,-35.000000") "TraceTypeQuery2" false 0 "ForDuration" true "(R=1.000000,G=0.000000,B=0.000000,A=1.000000)" "(R=0.000000,G=1.000000,B=0.000000,A=1.000000)" (Variables|Detection|DetectDistance|GetDistanceDetectionFrequency)))
      (Variables|Detection|DetectDistance|SetDistanceToGroin 0.0)
      (if (== (.HitActor (Collision|BreakHitResult _outhit_3)) (Variables|BlackboardValues|GetSensedActor))
        (Variables|Detection|DetectDistance|SetDistanceToGroin (.Distance (Collision|BreakHitResult _outhit_3)))))
    (:then_3
      ;[1 1 1] After all distances have been gathered get max. If we took Min it would be harder to judge if trace has worked correctly. The difference between those lengths is minimal so it doesn't impact further actions in meaningfull way
      (bind _output_get (Variables|BlackboardValues|SetDistanceToPlayerValue (Math|Float|Max(Float) (Variables|Detection|DetectDistance|GetDistanceToHead) (Variables|Detection|DetectDistance|GetDistanceToChest) (Variables|Detection|DetectDistance|GetDistanceToGroin))))
      (return _output_get))))