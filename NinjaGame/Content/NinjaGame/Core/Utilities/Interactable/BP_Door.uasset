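; BP_Door is an interactable double door that toggles between open and closed, either directly or remotely depending on its RemoteActivation flag.
; Both interaction events share a FlipFlop that plays or reverses the Door timeline, whose rate derives from DoorOpeningTime.
; MoveDoorWings interpolates yaw from the right wing's starting rotation, mirroring it for the left wing.
; Box overlaps report actors entering or leaving interaction range.
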(event OnComponentBeginOverlap(Box)
  (params (OverlappedComponent :type Primitive%20Component%20Object%20Reference) (OtherActor :type Actor%20Object%20Reference) (OtherComp :type Primitive%20Component%20Object%20Reference) (OtherBodyIndex :type Integer) (bFromSweep :type Boolean) (SweepResult :type Hit%20Result%20Structure%20%28by%20ref%29))
  (Utilities|IsinInteractionRange OtherActor))

(event OnComponentEndOverlap(Box)
  (params (OverlappedComponent :type Primitive%20Component%20Object%20Reference) (OtherActor :type Actor%20Object%20Reference) (OtherComp :type Primitive%20Component%20Object%20Reference) (OtherBodyIndex :type Integer))
  (Utilities|IsOutOfInteractionRange OtherActor))

(event EventInteractRemotely
  (if (Variables|Settings|GetRemoteActivation)
    (Utilities|FlowControl|FlipFlop
      (:A
        (bind _doormovement (Timeline|Door Play)
          (:Update
            (CallFunction|MoveDoorWings _doormovement))))
      (:B
        (Timeline|Door Reverse)))))

(event EventInteract
  (params (OtherActor :type Actor%20Object%20Reference))
  (if (not (Variables|Settings|GetRemoteActivation))
    (Utilities|FlowControl|FlipFlop
      (:A
        (bind _doormovement (Timeline|Door Play)
          (:Update
            (CallFunction|MoveDoorWings _doormovement))))
      (:B
        (Timeline|Door Reverse)))))

(event EventBeginPlay
  (Components|Timeline|SetPlayRate (Variables|Default|GetDoor) (/ 1.0 (Variables|Settings|GetDoorOpeningTime)))
  (Variables|InitialSettings|SetWingsStartRotation (.yaw (Variables|/Script/Engine.SceneComponent|GetRelativeRotation (Variables|Default|GetDoorRight)))))

(fn ConstructionScript)

(fn MoveDoorWings
  (params (Alpha :type Float%20%28double-precision%29))
  (bind _wingsstartrotation (Variables|InitialSettings|GetWingsStartRotation))
  (bind _wingsendrotation (Variables|Settings|GetWingsEndRotation))
  (bind _returnvalue (+ _wingsstartrotation _wingsendrotation))
  (bind _returnvalue_2 (Math|Float|Lerp _wingsstartrotation _returnvalue Alpha))
  (Transformation|SetRelativeRotation (Variables|Default|GetDoorRight) (Math|Rotator|MakeRotator 0.0 0.0 _returnvalue_2) false false)
  (Transformation|SetRelativeRotation (Variables|Default|GetDoorLeft) (Math|Rotator|MakeRotator 0.0 0.0 (* _returnvalue_2 -1.0)) false false))