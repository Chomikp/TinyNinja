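; BP_Button is an interactable button that triggers a paired actor, such as a door, through a remote interact message.
; Interacting while overlapping its Box plays a timeline that slides the mesh along X.
; Manual mode toggles on each interaction, while Automatic mode schedules a timed reverse.
; Timeline completion in either direction flips Pushed and messages the paired actor, with the Pushed check stopping the automatic cycle repeating.
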(event OnComponentBeginOverlap(Box)
  (params (OverlappedComponent :type Primitive%20Component%20Object%20Reference) (OtherActor :type Actor%20Object%20Reference) (OtherComp :type Primitive%20Component%20Object%20Reference) (OtherBodyIndex :type Integer) (bFromSweep :type Boolean) (SweepResult :type Hit%20Result%20Structure%20%28by%20ref%29))
  (Utilities|IsinInteractionRange OtherActor))

(event OnComponentEndOverlap(Box)
  (params (OverlappedComponent :type Primitive%20Component%20Object%20Reference) (OtherActor :type Actor%20Object%20Reference) (OtherComp :type Primitive%20Component%20Object%20Reference) (OtherBodyIndex :type Integer))
  (Utilities|IsOutOfInteractionRange OtherActor))

(event Custom|Reverse%20Button
  ;[1 1 1] Remote Button Logic
  (if (Variables|Bools|GetPushed)
    (bind _buttonmovementalpha (Timeline|ButtonRemote Reverse)
      (:Update
        (CallFunction|MoveButton _buttonmovementalpha))
      (:Finished
        (Utilities|Time|SetTimerbyEvent (delegate Custom|Reverse%20Button) (Variables|Settings|GetTimer))
        (CallFunction|NegatePushed)
        (CallFunction|MoveDoor)))))

(event EventBeginPlay
  (Variables|InitialSettings|SetStartLocation (.x (Variables|/Script/Engine.SceneComponent|GetRelativeLocation (Variables|Default|GetButton)))))

(event EventInteract
  (params (OtherActor :type Actor%20Object%20Reference))
  (if (Collision|IsOverlappingActor (Variables|Default|GetBox) OtherActor :!class /Script/Engine.PrimitiveComponent)
    (if (not (Variables|Bools|GetAutomatic))
      ;[1 1 1] Manual Button Logic
      (if (not (Variables|Bools|GetPushed))
        (bind _buttonmovementalpha (Timeline|ButtonManual Play)
          (:Update
            (CallFunction|MoveButton _buttonmovementalpha))
          (:Finished
            (CallFunction|NegatePushed)
            (CallFunction|MoveDoor)))
        (else
          (Timeline|ButtonManual Reverse)))
      (else
        ;[1 1 1] Remote Button Logic
        (if (not (Variables|Bools|GetPushed))
          (bind _buttonmovementalpha_2 (Timeline|ButtonRemote Play)
            (:Update
              (CallFunction|MoveButton _buttonmovementalpha_2))
            (:Finished
              (Utilities|Time|SetTimerbyEvent (delegate Custom|Reverse%20Button) (Variables|Settings|GetTimer))
              (CallFunction|NegatePushed)
              (CallFunction|MoveDoor))))))))

(fn ConstructionScript)

(fn MoveButton
  (params (Alpha :type Float%20%28double-precision%29))
  (bind _startlocation (Variables|InitialSettings|GetStartLocation))
  (Transformation|SetRelativeLocation (Variables|Default|GetButton) (Math|Vector|MakeVector (Math|Float|Lerp _startlocation (+ _startlocation -2e+01) Alpha) 0.0 0.0) false false))

(fn NegatePushed
  (Variables|Bools|SetPushed (not (Variables|Bools|GetPushed))))

(fn MoveDoor
  (bind _pairedactor (Variables|Settings|GetPairedActor))
  (Utilities|IsValid _pairedactor
    (:Is%20Valid
      (Class|BPIInteractable|InteractRemotely(Message) _pairedactor))))