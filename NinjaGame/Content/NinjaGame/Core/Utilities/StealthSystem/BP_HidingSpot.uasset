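; BP_HidingSpot is an unfinished stealth hiding-spot actor with a Box trigger meant to mark when the player is hidden.
; Begin overlap compares the actor to PlayerCharacter but takes no action, and the "Hidden" print and InHidingSpotEvent call are disconnected.
; End overlap prints "Not Hidden" for the player pawn and casts it to BP_PlayerCharacter without using the result.
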(event OnComponentBeginOverlap(Box)
  (params (OverlappedComponent :type Primitive%20Component%20Object%20Reference) (OtherActor :type Actor%20Object%20Reference) (OtherComp :type Primitive%20Component%20Object%20Reference) (OtherBodyIndex :type Integer) (bFromSweep :type Boolean) (SweepResult :type Hit%20Result%20Structure%20%28by%20ref%29))
  (if (== OtherActor (Variables|Default|GetPlayerCharacter))
    _))

(event OnComponentEndOverlap(Box)
  (params (OverlappedComponent :type Primitive%20Component%20Object%20Reference) (OtherActor :type Actor%20Object%20Reference) (OtherComp :type Primitive%20Component%20Object%20Reference) (OtherBodyIndex :type Integer))
  (bind _returnvalue (Game|GetPlayerCharacter 0))
  (if (== OtherActor _returnvalue)
    (Development|PrintString "Not Hidden")
    (Utilities|Casting|CastToBP_PlayerCharacter _returnvalue)))

(event EventBeginPlay)

(fn ConstructionScript)