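; BP_Enemy_Basic_StateTreeTest is a basic enemy character, named as a StateTree test, with simple health, damage and patrol support.
; It starts at max health, subtracts clamped damage and destroys itself at zero.
; A WasHit flag, set and reset by events, blocks repeat damage within one attack.
; Helper functions set walk speed and step cyclically through the waypoint array in ACPatrolWaypoints.
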(event Custom|DestroyThisActor
  (Actor|DestroyActor))

(event Game|Damage|EventAnyDamage
  (params (Damage :type Float%20%28single-precision%29) (DamageType :type Damage%20Type%20Object%20Reference) (InstigatedBy :type Controller%20Object%20Reference) (DamageCauser :type Actor%20Object%20Reference))
  ;[1 1 1] Simple take damage system
  (if (not (Variables|Default|GetWasHit))
    (bind _output_get (Variables|Default|SetCurrentHealth (Math|Float|Clamp(Float) (- (Variables|Default|GetCurrentHealth) Damage) 0.0 (Variables|Default|GetMaxHealth))))
    (if (== _output_get 0.0)
      (CallFunction|DestroyThisActor))))

(event EventBeginPlay
  (Variables|Default|SetCurrentHealth (Variables|Default|GetMaxHealth)))

(event EventResetActorsHitwithThisAttack
  ;[1 1 1] Allow this actor to be hit only once with each attack
  (Variables|Default|SetWasHit false))

(event EventWasHitwithThisAttack
  ;[1 1 1] Allow this actor to be hit only once with each attack
  (Variables|Default|SetWasHit true))

(fn ConstructionScript)

(fn UpdateWalkSpeed
  (params (NewWalkSpeed :type Float%20%28double-precision%29))
  (Variables|/Script/Engine.CharacterMovementComponent|SetMaxWalkSpeed (Variables|Character|GetCharacterMovement) NewWalkSpeed))

(fn GetNextWaypoint
  (bind _ac_patrolwaypoints (Variables|Default|GetAC_PatrolWaypoints))
  (bind _patrolwaypointarray (Variables|/Game/NinjaGame/Core/Enemies/StateTreeTest/AC_PatrolWaypoints.AC_PatrolWaypoints_C|GetPatrolWaypointArray _ac_patrolwaypoints))
  (Variables|Patrol|SetWaypointLocation (Transformation|GetActorLocation (Utilities|Array|Get(acopy) _patrolwaypointarray (Variables|Patrol|GetIndex))))
  (if (< (Variables|Patrol|GetIndex) (- (Utilities|Array|Length _patrolwaypointarray) 1))
    (Math|Integer|IncrementInt (Variables|Patrol|GetIndex))
    (else
      (Variables|Patrol|SetIndex 0))))